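; Lobby game mode that admits players, manages character selection and host map settings, then server-travels everyone to the chosen arena.
; PostLogin initializes each lobby controller with server details from the game instance, while players over the limit are kicked on a timer.
; UpdateClients pushes the roster and available characters to every controller and derives CanStart from character and ready status.
; Character swaps respawn at random PlayerStarts, and logout frees the leaver's character.
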(event `KickExtraPlayers`
  (for _array_element (`self.ExtraPlayers`)
    (`/Engine/EditorBlueprintResources/StandardMacros.IsValid` _array_element
      (:`Is Valid`
        (bind _asbp_lobby_player_controller (cast `/Game/MultiplayerGame/Blueprints/Lobby/BP_LobbyPlayerController` _array_element))
        (`/Game/MultiplayerGame/Blueprints/Lobby/BP_LobbyPlayerController.Kicked` _asbp_lobby_player_controller "Host is Full.")))))

(event `self.K2_PostLogin`
  (params (NewPlayer :type "PlayerController Object Reference"))
  (bind _maxplayer (`self.MaxPlayer`))
  (bind _asbp_game_instance (cast `/Game/MultiplayerGame/Blueprints/General/BP_GameInstance` (`GameplayStatics.GetGameInstance`) :!pure true))
  (if (and (>= (`self.CurrentPlayer`) _maxplayer) (!= _maxplayer 0))
    (`KismetArrayLibrary.Array_Add` (`self.ExtraPlayers`) NewPlayer)
    (`KismetSystemLibrary.K2_SetTimerDelegate` (delegate `KickExtraPlayers`) 2.0 true)
    (else
      (`KismetArrayLibrary.Array_Add` (`self.ConnectedPlayers`) NewPlayer)
      (set `self.MaxPlayer` (`/Game/MultiplayerGame/Blueprints/General/BP_GameInstance.MaxPlayer` _asbp_game_instance))
      (set `self.ServerName` (`/Game/MultiplayerGame/Blueprints/General/BP_GameInstance.ServerName` _asbp_game_instance))
      (if (== (`KismetArrayLibrary.Array_Length` (`self.SpawnPoints`)) 0)
        (bind _outactors (`GameplayStatics.GetAllActorsOfClass` "/Script/Engine.PlayerStart"))
        (set `self.SpawnPoints` _outactors))
      (bind _asbp_lobby_player_controller (cast `/Game/MultiplayerGame/Blueprints/Lobby/BP_LobbyPlayerController` NewPlayer))
      (`/Game/MultiplayerGame/Blueprints/Lobby/BP_LobbyPlayerController.InitialPlayerInfo` _asbp_lobby_player_controller)
      (`/Game/MultiplayerGame/Blueprints/Lobby/BP_LobbyPlayerController.CreateLobbyMenu` _asbp_lobby_player_controller (`self.ServerName`))
      (`/Game/MultiplayerGame/Blueprints/Lobby/BP_LobbyPlayerController.UpdateLobbySettings` _asbp_lobby_player_controller (`self.Map Image`) (`self.Map Name`) (`self.Map Time`))
      (`self.UpdateClients`))))

(event `SwapCharacter`
  (params (PlayerController :type "PlayerController Object Reference") (CharacterClass :type "/Game/MultiplayerGame/Blueprints/Character/BP_BaseCharacter Class Reference"))
  (bind _returnvalue (`Controller.K2_GetPawn` PlayerController))
  (bind _spawnpoints (`self.SpawnPoints`))
  (`/Engine/EditorBlueprintResources/StandardMacros.IsValid` _returnvalue
    (:`Is Valid`
      (`self.K2_DestroyActor` _returnvalue))
    (:`Is Not Valid`
      _))
  (bind _returnvalue_2 (`|SpawnActorFromClass` CharacterClass (`self.GetTransform` (`|GetArrayItem` _spawnpoints (`KismetMathLibrary.RandomIntegerInRange` 0 (- (`KismetArrayLibrary.Array_Length` _spawnpoints) 1)))) "Undefined" "OverrideRootScale" null null))
  (`Controller.Possess` PlayerController _returnvalue_2))

(event `UpdateClients`
  (bind _connectedplayers (`self.ConnectedPlayers`))
  (bind _output_get (set `self.CurrentPlayer` (`KismetArrayLibrary.Array_Length` (`self.ConnectedPlayers`))))
  (if (> _output_get 0)
    (`KismetArrayLibrary.Array_Clear` (`self.ConnectedPlayersInfo`))
    (for _array_element _connectedplayers
      (bind _asbp_lobby_player_controller (cast `/Game/MultiplayerGame/Blueprints/Lobby/BP_LobbyPlayerController` _array_element))
      (`KismetArrayLibrary.Array_Add` (`self.ConnectedPlayersInfo`) (`/Game/MultiplayerGame/Blueprints/Lobby/BP_LobbyPlayerController.PlayerInfo` _asbp_lobby_player_controller))
      (`/Game/MultiplayerGame/Blueprints/Lobby/BP_LobbyPlayerController.UpdatePlayerNumDisplayText` _asbp_lobby_player_controller (`self.CurrentPlayer`) (`self.MaxPlayer`)))
    (for _array_element_2 _connectedplayers
      (bind _asbp_lobby_player_controller_2 (cast `/Game/MultiplayerGame/Blueprints/Lobby/BP_LobbyPlayerController` _array_element_2))
      (`/Game/MultiplayerGame/Blueprints/Lobby/BP_LobbyPlayerController.UpdatePlayerInfoList` _asbp_lobby_player_controller_2 (`self.ConnectedPlayersInfo`))
      (`/Game/MultiplayerGame/Blueprints/Lobby/BP_LobbyPlayerController.UpdateAvailableCharacters` _asbp_lobby_player_controller_2 (`self.AvailableCharacters`))
      (`self.UpdateKickList`))
    (for _array_element_3 (`self.ConnectedPlayersInfo`)
      (if (or (== (`.CharacterClass_8_0C17D36749A6574C7F5B409C36D0190F` (break `/Game/MultiplayerGame/Blueprints/General/FPlayerInfo` _array_element_3)) "/Game/MultiplayerGame/Blueprints/Character/BP_BaseCharacter.BP_BaseCharacter_C") (`|EnumEquality` (`.ReadyStatus_14_D8198DBD416D1DB9E63AA3B0D4B729FF` (break `/Game/MultiplayerGame/Blueprints/General/FPlayerInfo` _array_element_3)) "NewEnumerator1"))
        (set `self.CanStart` false)
        (break)
        (else
          (set `self.CanStart` true))))))

(event `UpdateKickList`
  (bind _asbp_lobby_player_controller (cast `/Game/MultiplayerGame/Blueprints/Lobby/BP_LobbyPlayerController` (`GameplayStatics.GetPlayerController` 0)))
  (bind _lobbymenuref (`/Game/MultiplayerGame/Blueprints/Lobby/BP_LobbyPlayerController.LobbyMenuRef` _asbp_lobby_player_controller))
  (`/Engine/EditorBlueprintResources/StandardMacros.IsValid` _lobbymenuref
    (:`Is Valid`
      (bind _gamesettingswindow (`/Game/MultiplayerGame/Blueprints/Widget/Lobby/WBP_LobbyMenu.GameSettingsWindow` _lobbymenuref))
      (if (`Widget.IsVisible` _gamesettingswindow)
        (`/Game/MultiplayerGame/Blueprints/Widget/Lobby/WBP_GameSettingsWindow.UpdatePlayerList` _gamesettingswindow)))))

(event `StartGame`
  (bind _returnvalue (`GameplayStatics.GetPlayerController` 0))
  (set `/Game/MultiplayerGame/Blueprints/General/BP_GameInstance.MapTime` (`self.Map Time`) (cast `/Game/MultiplayerGame/Blueprints/General/BP_GameInstance` (`GameplayStatics.GetGameInstance`) :!pure true))
  (switch `int` (`self.MapID`)
    (:`0`
      (`KismetSystemLibrary.ExecuteConsoleCommand` "servertravel /Game/MultiplayerGame/Maps/Arena01" _returnvalue))
    (:`1`
      (`KismetSystemLibrary.ExecuteConsoleCommand` "servertravel /Game/MultiplayerGame/Maps/Arena02" _returnvalue))))

(event `UpdateGameSettings`
  (params (MapImage :type "Texture2D Object Reference") (MapName :type Text) (MapTime :type Text) (MapID :type Integer))
  (set `self.Map Image` MapImage)
  (set `self.Map Name` MapName)
  (set `self.Map Time` MapTime)
  (set `self.MapID` MapID)
  (for _array_element (`self.ConnectedPlayers`)
    (bind _asbp_lobby_player_controller (cast `/Game/MultiplayerGame/Blueprints/Lobby/BP_LobbyPlayerController` _array_element))
    (`/Game/MultiplayerGame/Blueprints/Lobby/BP_LobbyPlayerController.UpdateLobbySettings` _asbp_lobby_player_controller (`self.Map Image`) (`self.Map Name`) (`self.Map Time`))))

(event `KickPlayer`
  (params (PlayerIndex :type Integer))
  (bind _asbp_lobby_player_controller (cast `/Game/MultiplayerGame/Blueprints/Lobby/BP_LobbyPlayerController` (`|GetArrayItem` (`self.ConnectedPlayers`) PlayerIndex)))
  (`/Game/MultiplayerGame/Blueprints/Lobby/BP_LobbyPlayerController.Kicked` _asbp_lobby_player_controller "You Got Kicked."))

(event `self.K2_OnLogout`
  (params (ExitingController :type "Controller Object Reference"))
  (bind _connectedplayers (`self.ConnectedPlayers`))
  (bind `_as玩家控制器` (cast `PlayerController` ExitingController))
  (bind _returnvalue (`KismetArrayLibrary.Array_Find` _connectedplayers `_as玩家控制器`))
  (bind _asbp_lobby_player_controller (cast `/Game/MultiplayerGame/Blueprints/Lobby/BP_LobbyPlayerController` (`|GetArrayItem` _connectedplayers _returnvalue)))
  (`KismetArrayLibrary.Array_Set` (`self.AvailableCharacters`) (`/Game/MultiplayerGame/Blueprints/Lobby/BP_LobbyPlayerController.CurrentSelectCharacterIndex` _asbp_lobby_player_controller) true)
  (`KismetArrayLibrary.Array_Remove` (`self.ConnectedPlayers`) _returnvalue)
  (`KismetArrayLibrary.Array_Remove` (`self.ConnectedPlayersInfo`) _returnvalue)
  (`self.UpdateClients`))

(fn `UserConstructionScript`)