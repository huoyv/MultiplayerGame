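; BP_RoomGameMode is the game mode for a multiplayer room, tracking connected players and handling their respawns.
; On controller swap it registers the new controller, copies PlayerInfo from the lobby controller to the room controller and shows the Game Instance's map time.
; RespawnCharacter destroys the current pawn, then spawns and possesses the requested class at a random cached PlayerStart.
; Logout removes the player from the list and calls LeaveGame on the Game Instance.
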(event `self.K2_OnSwapPlayerControllers`
  (params (OldPC :type "PlayerController Object Reference") (NewPC :type "PlayerController Object Reference"))
  (`KismetArrayLibrary.Array_Add` (`self.ConnectedPlayers`) NewPC)
  (bind _asbp_room_player_controller (cast `/Game/MultiplayerGame/Blueprints/Gameplay/BP_RoomPlayerController` NewPC))
  (bind _asbp_lobby_player_controller (cast `/Game/MultiplayerGame/Blueprints/Lobby/BP_LobbyPlayerController` OldPC))
  (set `/Game/MultiplayerGame/Blueprints/Gameplay/BP_RoomPlayerController.PlayerInfo` (`/Game/MultiplayerGame/Blueprints/Lobby/BP_LobbyPlayerController.PlayerInfo` _asbp_lobby_player_controller) _asbp_room_player_controller)
  (`/Game/MultiplayerGame/Blueprints/Gameplay/BP_RoomPlayerController.ShowMapTime` _asbp_room_player_controller (`/Game/MultiplayerGame/Blueprints/General/BP_GameInstance.MapTime` (cast `/Game/MultiplayerGame/Blueprints/General/BP_GameInstance` (`GameplayStatics.GetGameInstance`) :!pure true))))

(event `RespawnCharacter`
  (params (PlayerController :type "PlayerController Object Reference") (CharacterClass :type "/Game/MultiplayerGame/Blueprints/Character/BP_BaseCharacter Class Reference"))
  (bind _returnvalue (`Controller.K2_GetPawn` PlayerController))
  (bind _spawnpoints (`self.SpawnPoints`))
  (if (== (`KismetArrayLibrary.Array_Length` (`self.SpawnPoints`)) 0)
    (bind _outactors (`GameplayStatics.GetAllActorsOfClass` "/Script/Engine.PlayerStart"))
    (set `self.SpawnPoints` _outactors))
  (`/Engine/EditorBlueprintResources/StandardMacros.IsValid` _returnvalue
    (:`Is Valid`
      (`self.K2_DestroyActor` _returnvalue))
    (:`Is Not Valid`
      _))
  (bind _returnvalue_2 (`|SpawnActorFromClass` CharacterClass (`self.GetTransform` (`|GetArrayItem` _spawnpoints (`KismetMathLibrary.RandomIntegerInRange` 0 (- (`KismetArrayLibrary.Array_Length` _spawnpoints) 1)))) "Undefined" "OverrideRootScale" null null))
  (`Controller.Possess` PlayerController _returnvalue_2))

(event `self.K2_OnLogout`
  (params (ExitingController :type "Controller Object Reference"))
  (bind _connectedplayers (`self.ConnectedPlayers`))
  (bind _asplayer_controller (cast `PlayerController` ExitingController))
  (`KismetArrayLibrary.Array_Remove` _connectedplayers (`KismetArrayLibrary.Array_Find` _connectedplayers _asplayer_controller))
  (`/Game/MultiplayerGame/Blueprints/General/BP_GameInstance.LeaveGame` (cast `/Game/MultiplayerGame/Blueprints/General/BP_GameInstance` (`GameplayStatics.GetGameInstance`) :!pure true) _asplayer_controller))

(fn `UserConstructionScript`)